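; Win trigger volume that completes the level when the player overlaps it and no BP_Crystal actors remain in the world.
; The crystal check queries all actors of that class on each player overlap, printing a message if any are left.
; Progression finds the current level in the ordered LevelNames array and opens the next by name, or prints a game-complete message on the final entry.
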(event EventBeginPlay)

(event Collision|EventActorBeginOverlap
  (params (OtherActor :type Actor%20Object%20Reference))
  (Utilities|IsPlayer OtherActor
    (:IsPlayer
      (if (CallFunction|AnyCrystalsRemain)
        (Development|PrintString "CRYSTALS REMAIN")
        (else
          (LevelManagement|CompleteLevel))))))

(fn ConstructionScript)

(fn AnyCrystalsRemain
  (bind _outactors (Actor|GetAllActorsOfClass "/Game/Blueprints/BP_Crystal.BP_Crystal_C"))
  (return (> (Utilities|Array|Length _outactors) 0)))

(fn GetCurrentLevelIndex
  (bind _returnvalue (Game|GetCurrentLevelName true))
  (return (Utilities|Array|FindItem (Variables|Default|GetLevelNames) (Utilities|String|StringToName _returnvalue))))

(fn CompleteLevel
  (if (LevelManagement|IsFinalLevel)
    (Development|PrintString "GAME COMPLETE")
    (else
      (LevelManagement|LoadNextLevel))))

(fn IsFinalLevel
  (return (== (LevelManagement|GetCurrentLevelIndex) (Utilities|Array|LastIndex (Variables|Default|GetLevelNames)))))

(fn LoadNextLevel
  (Game|OpenLevel(byName) (LevelManagement|GetNextLevelName)))

(fn GetNextLevelName
  (return (Utilities|Array|Get(acopy) (Variables|Default|GetLevelNames) (+ (LevelManagement|GetCurrentLevelIndex) 1))))