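; BP_Crystal is a collectible crystal that the player picks up by overlapping it.
; On pickup it caches its location, scale and light intensity, then plays a pitch-randomized sound and prints a debug message.
; A timeline moves it toward the player's live position while animating scale and point-light intensity from a shared curve, then destroys it.
; The orb counter increment is unwired, so pickups are not counted.
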(event Collision|EventActorBeginOverlap
  (params (OtherActor :type Actor%20Object%20Reference))
  (Utilities|IsPlayer OtherActor
    (:IsPlayer
      (CallFunction|SetStartValues)
      (Audio|PlaySound2D "/Game/Sounds/S_SandSwish_CollectCrystal.S_SandSwish_CollectCrystal" 1.0 (Math|Random|RandomFloatinRange 0.9 1.1) 0.0 0 0)
      (Development|PrintString "Orb collected!" true true "(R=0.000000,G=0.852485,B=1.000000,A=1.000000)")
      (bind (_direction _alpha_zerotoone _alpha_scaleupbeforezero) (Timeline|CollectionTimeline Play)
        (:Update
          (CallFunction|MovetoPlayer _alpha_zerotoone)
          (CallFunction|ScaletoZero _alpha_scaleupbeforezero _alpha_zerotoone)
          (CallFunction|LightSurge _alpha_scaleupbeforezero))
        (:Finished
          (Actor|DestroyActor))))))

(fn ConstructionScript)

(fn MovetoPlayer
  (params (Alpha :type Float%20%28single-precision%29))
  (Transformation|SetActorLocation (Math|Vector|Lerp(Vector) (Variables|Default|GetStartLocation) (Transformation|GetActorLocation (Game|Player|GetPlayerPawn 0)) Alpha) false true))

(fn SetStartValues
  (Variables|Default|SetStartLocation (Transformation|GetActorLocation))
  (Variables|Default|SetStartScale (Transformation|GetActorScale3D))
  (Variables|Default|SetStartPointLightIntensity (Variables|/Script/Engine.LightComponentBase|GetIntensity (Variables|Default|GetPointLight))))

(fn ScaletoZero
  (params (InFloat :type Float%20%28single-precision%29) (Alpha :type Float%20%28single-precision%29))
  (Transformation|SetActorScale3D (Math|Vector|Lerp(Vector) (Variables|Default|GetStartScale) (Math|Conversions|ToVector(Float) InFloat) Alpha)))

(fn LightSurge
  (params (A :type Float%20%28single-precision%29))
  (Rendering|Components|Light|SetIntensity (Variables|Default|GetPointLight) (* A (Variables|Default|GetStartPointLightIntensity))))