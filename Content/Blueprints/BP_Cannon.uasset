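; BP_Cannon is a cannon actor that automatically and intermittently fires projectiles from its Arrow component.
; From BeginPlay it loops on a FireRate delay, spawning a scaled BP_Projectile each cycle.
; A random boolean either plays a timeline that moves the barrel along local Y, or immediately destroys the new projectile.
; The loop re-enters the Delay from timeline updates or straight after the destroy.
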(event EventBeginPlay
  (bind _arrow (Variables|Default|GetArrow))
  (Utilities|FlowControl|Delay (Variables|CannonProperties|GetFireRate) :!label _label)
  (bind _returnvalue (Game|SpawnActorfromClass "/Game/Blueprints/BP_Projectile.BP_Projectile_C" (Math|Transform|MakeTransform (Transformation|GetWorldLocation _arrow) (Transformation|GetWorldRotation _arrow) (Math|Conversions|ToVector(Float) (Variables|CannonProperties|GetProjectileScale))) "Undefined" 0 0))
  (if (Math|Random|RandomBool)
    (bind _barrellocationonfire (Timeline|Timeline_0 PlayFromStart)
      (:Update
        (CallFunction|MoveCannonBarrel _barrellocationonfire)
        (goto _label)))
    (else
      (Actor|DestroyActor _returnvalue)
      (goto _label))))

(fn ConstructionScript)

(fn MoveCannonBarrel
  (params (CannonBarrel_LocationY :type Float%20%28single-precision%29))
  (Transformation|SetRelativeLocation (Variables|Default|GetCannon_Barrel) (Math|Vector|MakeVector 0.0 CannonBarrel_LocationY 0.0) false false))